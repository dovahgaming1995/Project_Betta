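; Meltable metal actor that plays a one-shot melting animation when it detects an active BP_Flames actor.
; Every tick runs a server event that multicasts a Visibility box trace just above the MeltingMetal mesh.
; When the hit actor is BP_Flames with ActivateMeltingMetal set, a DoOnce plays the non-looping animation.
; Detection is polled through per-frame RPCs rather than overlap events.
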(event Custom|Multicast_Tick
  (bind _melting_metal (Variables|Default|GetMelting_Metal))
  (bind _returnvalue (Transformation|GetWorldLocation _melting_metal))
  ;[0.177 1 0] Check at all times whether someone or "BP_Flames" is on the scene. If so, check if "Activate Melting Metal" is true. If everything is ok, activate the animation.
  (bind (_outhit _returnvalue_2) (Collision|BoxTraceByChannel (+ _returnvalue "0, 0,55.000000") (+ _returnvalue "5.000000,5.000000,55.000000") "150.000000,150.000000,50.000000" "0, 0, 0" "TraceTypeQuery1" false 0 "None"))
  (if _returnvalue_2
    (bind _asbp_flames (Utilities|Casting|CastToBP_Flames (.HitActor (Collision|BreakHitResult _outhit))))
    (if (Variables|/Game/SuperPowers/Characters/Blueprints/BP_Flames.BP_Flames_C|GetActivate%20Melting%20Metal _asbp_flames)
      (Utilities|FlowControl|DoOnce false
        (:Completed
          (Components|Animation|PlayAnimation (Variables|Default|GetMelting_Metal) "/Game/SuperPowers/Maps/Melting_Metal/Melting_Metal_Anim.Melting_Metal_Anim" false))))))

(event Custom|RunOnServer_Tick
  ;[0.177 1 0] Check at all times whether someone or "BP_Flames" is on the scene. If so, check if "Activate Melting Metal" is true. If everything is ok, activate the animation.
  (CallFunction|MulticastTick))

(event EventTick
  (params (DeltaSeconds :type Float%20%28single-precision%29))
  ;[0.177 1 0] Check at all times whether someone or "BP_Flames" is on the scene. If so, check if "Activate Melting Metal" is true. If everything is ok, activate the animation.
  (CallFunction|RunonServerTick))

(fn ConstructionScript)