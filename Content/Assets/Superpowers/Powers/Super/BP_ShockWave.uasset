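; BP_ShockWave is a superpower effect actor that shows an expanding shockwave mesh with sound.
; On BeginPlay, the Size timeline adds its Scale track to the mesh's world scale every update.
; When the timeline finishes, the mesh is destroyed, and the actor follows after a delay.
; An optional server optimization flag deactivates the sound on the authority, while remote instances keep it.
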(event EventBeginPlay
  (bind _mesh_shockwave (Variables|Default|GetMesh_ShockWave))
  ;[1 0 0] Optimize Server? If so, "Clients" will normally follow the path. "Server" will have sound effects disabled.
  (if (Variables|Server|GetEnable%20Advanced%20Server%20Optimization?)
    (Networking|SwitchHasAuthority
      (:Authority
        ;[1 1 1] Sound Effects
        (Components|Activation|SetActive (Variables|Default|GetS_ShockWave) false false)
        ;[1 0.9571 0] Increase the size of the ShockWave Mesh based on the values of the "Timeline" called "Scale".
        (bind _scale (Timeline|Size PlayFromStart)
          (:Update
            (Transformation|SetWorldScale3D _mesh_shockwave (+ (Transformation|GetWorldScale _mesh_shockwave) _scale)))
          (:Finished
            ;;[1 1 1] Destroy Mesh
            (Components|DestroyComponent (Variables|Default|GetMesh_ShockWave))
            (Utilities|FlowControl|Delay 1e+01)
            ;;[1 0 0] Destroy Actor
            (Actor|DestroyActor))))
      (:Remote
        (Timeline|Size PlayFromStart)))
    (else
      (Timeline|Size PlayFromStart))))

(fn ConstructionScript)