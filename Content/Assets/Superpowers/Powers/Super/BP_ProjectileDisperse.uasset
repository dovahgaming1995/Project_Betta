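; BP_ProjectileDisperse is a short-lived dispersal effect actor in the Superpowers set.
; On BeginPlay, a timeline animates the relative scale of its Sphere component, and the actor destroys itself after a fixed delay.
; When advanced server optimization is enabled, the authority deactivates the SWind sound, leaving the audio to clients.
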(event EventBeginPlay
  ;[1 0 0] Optimize Server? If so, "Clients" will normally follow the path. "Server" will have sound effects disabled.
  (if (Variables|Server|GetEnable%20Advanced%20Server%20Optimization?)
    (Networking|SwitchHasAuthority
      (:Authority
        ;[1 1 1] Sound Effects
        (Components|Activation|SetActive (Variables|Default|GetS_Wind) false false))
      (:Remote
        _)))
  ;[1 0.8582 0] Set object scale according to time and after 2s destroy actor.
  (Utilities|FlowControl|Sequence
    (:then_0
      (bind _scale (Timeline|Sphere_Scale PlayFromStart)
        (:Update
          (Transformation|SetRelativeScale3D (Variables|Default|GetSphere) _scale))))
    (:then_1
      (Utilities|FlowControl|Delay 2.0)
      (Actor|DestroyActor))))

(fn ConstructionScript)