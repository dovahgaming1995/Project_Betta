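; Force field actor that materializes with animated material and sound, then is destroyed after a set number of sphere overlaps.
; Mesh hits flicker the material and sphere overlaps count damage, both relayed through server and multicast events.
; An optional optimization flag skips cosmetic effects on the server.
; A per-tick sphere trace flags BP_Speedster and restores the saved Pawn collision response once the trace is empty.
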(event OnComponentHit(Force_Field)
  (params (HitComponent :type Primitive%20Component%20Object%20Reference) (OtherActor :type Actor%20Object%20Reference) (OtherComp :type Primitive%20Component%20Object%20Reference) (NormalImpulse :type Vector :default "0, 0, 0") (Hit :type Hit%20Result%20Structure%20%28by%20ref%29))
  ;[0.9928 1 0] When a character or any object collides with "Collision" animate material using "Timeline" to create a weak effect in the protection generated by the wall.
  ;;[1 0 0] Optimize Server? If so, "Clients" will normally follow the path. "Server" will have no "Hit" effect.
  (if (Variables|Server|GetEnable%20Advanced%20Server%20Optimization?)
    (Networking|SwitchHasAuthority
      (:Remote
        _)))
  (CallFunction|RunonServerForceField))

(event OnComponentBeginOverlap(Sphere)
  (params (OverlappedComponent :type Primitive%20Component%20Object%20Reference) (OtherActor :type Actor%20Object%20Reference) (OtherComp :type Primitive%20Component%20Object%20Reference) (OtherBodyIndex :type Integer) (bFromSweep :type Boolean) (SweepResult :type Hit%20Result%20Structure%20%28by%20ref%29))
  ;[1 0 0] When the sum of collisions results in 10 the actor will be destroyed.
  (CallFunction|RunonServerSphere))

(event Custom|Multicast_Force_Field
  ;[0.9928 1 0] When a character or any object collides with "Collision" animate material using "Timeline" to create a weak effect in the protection generated by the wall.
  (bind _boost (Timeline|Weak%20Effect PlayFromStart)
    (:Update
      (Rendering|Material|SetScalarParameterValue (stale EventBeginPlay _returnvalue) "Boost" _boost :!class /Script/Engine.MaterialInstanceDynamic))))

(event Custom|Multicast_Sphere
  ;[1 0 0] When the sum of collisions results in 10 the actor will be destroyed.
  ;;[1 0 0] Optimize Server? If so, "Clients" will normally follow the path. "Server" will have dematerialization and sound effects disabled.
  (if (Variables|Server|GetEnable%20Advanced%20Server%20Optimization?)
    (Networking|SwitchHasAuthority
      (:Authority
        (bind _output_get (Variables|Hit|SetHit (+ (Variables|Hit|GetHit) 1) :!label _label))
        (if (>= _output_get (Variables|Hit|GetNumber%20of%20Hits%20for%20Destroy))
          ;;[1 0 0] Optimize Server? If so, "Clients" will normally follow the path. "Server" will have dematerialization and sound effects disabled.
          (if (Variables|Server|GetEnable%20Advanced%20Server%20Optimization?)
            (Networking|SwitchHasAuthority
              (:Authority
                (Utilities|FlowControl|Delay 1.0)
                (Actor|DestroyActor :!label _label_2))
              (:Remote
                ;;[1 1 1] Sound Effects
                (Components|Activation|SetActive (Variables|Default|GetS_LosingForce) true false :!label _label_3)
                (bind _losing_strength (Timeline|Losing%20Strength PlayFromStart)
                  (:Update
                    (Rendering|Material|SetScalarParameterValue (stale EventBeginPlay _returnvalue) "Opacity" _losing_strength :!class /Script/Engine.MaterialInstanceDynamic))
                  (:Finished
                    (goto _label_2)))))
            (else
              (goto _label_3)))))
      (:Remote
        ;;[1 1 1] Sound Effects
        (Components|Activation|SetActive (Variables|Default|GetS_TouchingTheForce) true false :!label _label_4)
        (Utilities|FlowControl|Sequence
          (:then_0
            (goto _label))
          (:then_1
            ;;[1 1 1] Sound Effects
            (Utilities|FlowControl|Delay 0.3)
            (Components|Activation|SetActive (Variables|Default|GetS_TouchingTheForce) false false)))))
    (else
      (goto _label_4))))

(event Custom|RunOnServer_Force_Field
  ;[0.9928 1 0] When a character or any object collides with "Collision" animate material using "Timeline" to create a weak effect in the protection generated by the wall.
  (CallFunction|MulticastForceField))

(event Custom|RunOnServer_Sphere
  ;[1 0 0] When the sum of collisions results in 10 the actor will be destroyed.
  (CallFunction|MulticastSphere))

(event EventBeginPlay
  ;[0.9928 1 0] Create Dynamic Material Instance to create Materialization Effect with changing values in the Parameters.
  ;;[1 1 1] Get "Sphere" collision configuration. Set Variable to save the configuration to be used in the "Sensor".
  (Variables|Vibrate|SetCollision (Collision|GetCollisionResponsetoChannel (Variables|Default|GetSphere) "ECC_Pawn"))
  ;;[1 0 0] Optimize Server? If so, "Clients" will normally follow the path. "Server" will have materialization and sound effects disabled.
  (if (Variables|Server|GetEnable%20Advanced%20Server%20Optimization?)
    (Networking|SwitchHasAuthority
      (:Authority
        ;;[1 1 1] Sound Effects
        (Components|Activation|SetActive (Variables|Default|GetS_Materialization) false false))
      (:Remote
        (bind _returnvalue (Rendering|Material|CreateDynamicMaterialInstance (Variables|Default|GetForce_Field) 0 0 :!class /Script/Engine.PrimitiveComponent :!label _label))
        (Utilities|FlowControl|Sequence
          (:then_0
            (bind (_direction _materializationz _boost _opacity) (Timeline|Materialization,%20Boost%20and%20Opacity PlayFromStart)
              (:Update
                (Rendering|Material|SetScalarParameterValue _returnvalue "Amount" _materializationz :!class /Script/Engine.MaterialInstanceDynamic)
                (Rendering|Material|SetScalarParameterValue _returnvalue "Boost" _boost :!class /Script/Engine.MaterialInstanceDynamic)
                (Rendering|Material|SetScalarParameterValue _returnvalue "Opacity" _opacity :!class /Script/Engine.MaterialInstanceDynamic))
              (:Finished
                ;;[1 1 1] Sound Effects
                (Utilities|FlowControl|Delay 2.0)
                (Components|Activation|SetActive (Variables|Default|GetS_Materialization) false false))))
          (:then_1
            ;;[1 1 1] Sound Effects
            (Utilities|FlowControl|Delay 0.2)
            (Components|Activation|SetActive (Variables|Default|GetS_Materialization) true false)))))
    (else
      (goto _label))))

(event EventTick
  (params (DeltaSeconds :type Float%20%28single-precision%29))
  (bind _sphere (Variables|Default|GetSphere))
  (bind _returnvalue (Transformation|GetWorldLocation _sphere))
  ;[0 0.9558 1] Create "Sensor" that will be updated at all times. The Sensor is detecting the character "Speedster". If the Speedster is detected, the Variable will be defined according to the result.
  (bind (_outhits _returnvalue_2) (Collision|MultiSphereTraceForObjects _returnvalue (+ _returnvalue "1.000000,1.000000,1.000000") 6.5e+02 (Utilities|Array|MakeArray "ObjectTypeQuery3") false 0 "None"))
  (if _returnvalue_2
    (for _array_element _outhits
      (Utilities|Casting|CastToBP_Speedster (.HitActor (Collision|BreakHitResult _array_element))
        (:then
          (Variables|Vibrate|SetCharacter%20Detected true))
        (:CastFailed
          (Variables|Vibrate|SetCharacter%20Detected false))))
    (else
      ;;[1 1 1 0] When the Character leaves the "Sensor", the "Sphere" collision will return to normal.
      (if (Variables|Vibrate|GetCharacter%20Detected)
        (Collision|SetCollisionResponsetoChannel (Variables|Default|GetSphere) "ECC_Pawn" (Variables|Vibrate|GetCollision))
        (Variables|Vibrate|SetCharacter%20Detected false)))))

(fn ConstructionScript)