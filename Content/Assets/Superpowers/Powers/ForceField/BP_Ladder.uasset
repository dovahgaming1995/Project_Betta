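; BP_Ladder is a Force Field power ladder that materializes on spawn and destroys itself shortly after an overlap with its Sensor ends.
; A timeline animates dynamic materials on ten steps alongside a sound, skipped on the server when advanced optimization is enabled.
; End overlap routes through server and multicast events to delayed destruction.
; Tick box-traces for BP_Speedster, setting CharacterDetected and restoring the Sensor's saved Pawn response once the trace clears.
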(event OnComponentEndOverlap(Sensor)
  (params (OverlappedComponent :type Primitive%20Component%20Object%20Reference) (OtherActor :type Actor%20Object%20Reference) (OtherComp :type Primitive%20Component%20Object%20Reference) (OtherBodyIndex :type Integer))
  ;[1 0.006725 0] After end of overlay destroy actor.
  (CallFunction|RunonServerSensor))

(event Custom|RunOnServer_Sensor
  ;[1 0.006725 0] After end of overlay destroy actor.
  (CallFunction|MulticastSensor))

(event Custom|Multicast_Sensor
  ;[1 0.006725 0] After end of overlay destroy actor.
  (Utilities|FlowControl|Delay 0.5)
  (Actor|DestroyActor))

(event EventBeginPlay
  ;[1 0.9326 0] Create Dynamic Material Instance to create Materialization Effect...
  ;;[1 1 1] Get "Sphere" collision configuration. Set Variable to save the configuration to be used in the "Sensor".
  (Variables|Vibrate|SetCollision (Collision|GetCollisionResponsetoChannel (Variables|Default|GetSensor) "ECC_Pawn"))
  ;;[1 0 0] Optimize Server? If so, "Clients" will normally follow the path. "Server" will have materialization and sound effects disabled.
  (if (Variables|Server|GetEnable%20Advanced%20Server%20Optimization?)
    (Networking|SwitchHasAuthority
      (:Remote
        _)))
  (Utilities|FlowControl|Sequence
    (:then_0
      (bind _returnvalue (Rendering|Material|CreateDynamicMaterialInstance (Variables|Default|GetStep1) 0 0 :!class /Script/Engine.PrimitiveComponent)))
    (:then_1
      (bind _returnvalue_2 (Rendering|Material|CreateDynamicMaterialInstance (Variables|Default|GetStep5) 0 0 :!class /Script/Engine.PrimitiveComponent)))
    (:then_2
      (bind _returnvalue_3 (Rendering|Material|CreateDynamicMaterialInstance (Variables|Default|GetStep2) 0 0 :!class /Script/Engine.PrimitiveComponent)))
    (:then_3
      (bind _returnvalue_4 (Rendering|Material|CreateDynamicMaterialInstance (Variables|Default|GetStep3) 0 0 :!class /Script/Engine.PrimitiveComponent)))
    (:then_4
      (bind _returnvalue_5 (Rendering|Material|CreateDynamicMaterialInstance (Variables|Default|GetStep4) 0 0 :!class /Script/Engine.PrimitiveComponent)))
    (:then_5
      (bind _returnvalue_6 (Rendering|Material|CreateDynamicMaterialInstance (Variables|Default|GetStep10) 0 0 :!class /Script/Engine.PrimitiveComponent)))
    (:then_6
      (bind _returnvalue_7 (Rendering|Material|CreateDynamicMaterialInstance (Variables|Default|GetStep6) 0 0 :!class /Script/Engine.PrimitiveComponent)))
    (:then_7
      (bind _returnvalue_8 (Rendering|Material|CreateDynamicMaterialInstance (Variables|Default|GetStep7) 0 0 :!class /Script/Engine.PrimitiveComponent)))
    (:then_8
      (bind _returnvalue_9 (Rendering|Material|CreateDynamicMaterialInstance (Variables|Default|GetStep8) 0 0 :!class /Script/Engine.PrimitiveComponent)))
    (:then_9
      (bind _returnvalue_10 (Rendering|Material|CreateDynamicMaterialInstance (Variables|Default|GetStep9) 0 0 :!class /Script/Engine.PrimitiveComponent)))
    (:then_10
      ;[1 0.9326 0] ...with changing values in the Parameters.
      (bind (_direction _materializationz _boost _opacity) (Timeline|Materialization,%20Boost%20and%20Opacity PlayFromStart)
        (:Update
          (Rendering|Material|SetScalarParameterValue _returnvalue "Amount" _materializationz :!class /Script/Engine.MaterialInstanceDynamic)
          (Rendering|Material|SetScalarParameterValue _returnvalue "Boost" _boost :!class /Script/Engine.MaterialInstanceDynamic)
          (Rendering|Material|SetScalarParameterValue _returnvalue "Opacity" _opacity :!class /Script/Engine.MaterialInstanceDynamic))
        (:Finished
          ;;[1 1 1] Sound Effects
          (Utilities|FlowControl|Delay 1.0)
          (Components|Activation|SetActive (Variables|Default|GetS_LadderMaterialization) false false))))
    (:then_11
      ;;[1 1 1] Sound Effects
      (Components|Activation|SetActive (Variables|Default|GetS_LadderMaterialization) true false))))

(event EventTick
  (params (DeltaSeconds :type Float%20%28single-precision%29))
  (bind _returnvalue (Transformation|GetActorLocation))
  (bind _returnvalue_2 (+ _returnvalue "500.000000, 0,200.000000"))
  ;[0 0.991 1] Create "Sensor" that will be updated at all times. The Sensor is detecting the character "Speedster". If the Speedster is detected, the Variable will be defined according to the result.
  (bind (_outhits _returnvalue_3) (Class|KismetSystemLibrary|BoxTraceMultiforObjects _returnvalue_2 (+ _returnvalue_2 "1.000000,1.000000,1.000000") "500.000000,100.000000,200.000000" (Transformation|GetActorRotation) (Utilities|Array|MakeArray "ObjectTypeQuery3") false 0 "None" true))
  (if _returnvalue_3
    (for _array_element _outhits
      (Utilities|Casting|CastToBP_Speedster (.HitActor (Collision|BreakHitResult _array_element))
        (:then
          (Variables|Vibrate|SetCharacter%20Detected true))
        (:CastFailed
          (Variables|Vibrate|SetCharacter%20Detected false))))
    (else
      ;;[1 1 1 0] When the Character leaves the "Sensor", the "Sphere" collision will return to normal.
      (if (Variables|Vibrate|GetCharacter%20Detected)
        (Collision|SetCollisionResponsetoChannel (Variables|Default|GetSensor) "ECC_Pawn" (Variables|Vibrate|GetCollision))
        (Variables|Vibrate|SetCharacter%20Detected false)))))

(fn ConstructionScript)