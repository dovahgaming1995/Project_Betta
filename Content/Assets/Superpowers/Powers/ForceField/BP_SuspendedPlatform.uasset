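; Suspended platform from the ForceField superpower that materializes on spawn and destroys itself after use.
; BeginPlay drives a timeline into a dynamic material and plays sound, optionally skipping both on the server.
; Tick box-traces for BP_Speedster, restoring the Sensor's saved Pawn collision response when the trace empties.
; Sensor end overlap, or every second Speedster exit via FlipFlop, triggers server-to-multicast delayed destruction.
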(event OnComponentEndOverlap(Sensor)
  (params (OverlappedComponent :type Primitive%20Component%20Object%20Reference) (OtherActor :type Actor%20Object%20Reference) (OtherComp :type Primitive%20Component%20Object%20Reference) (OtherBodyIndex :type Integer))
  ;[1 0 0] After end of overlay destroy actor.
  (CallFunction|RunonServerSensor))

(event Custom|Multicast_Sensor
  ;[1 0 0] After end of overlay destroy actor.
  (Utilities|FlowControl|Delay 0.5)
  (Actor|DestroyActor))

(event Custom|RunOnServer_Sensor
  ;[1 0 0] After end of overlay destroy actor.
  (CallFunction|MulticastSensor))

(event EventBeginPlay
  ;[1 1 1] Get "Sphere" collision configuration. Set Variable to save the configuration to be used in the "Sensor".
  (Variables|Collision|SetCollision%20Sensor (Collision|GetCollisionResponsetoChannel (Variables|Default|GetSensor) "ECC_Pawn"))
  ;[1 0 0] Optimize Server? If so, "Clients" will normally follow the path. "Server" will have materialization and sound effects disabled.
  (if (Variables|Server|GetEnable%20Advanced%20Server%20Optimization?)
    (Networking|SwitchHasAuthority
      (:Remote
        _)))
  ;[0.9968 1 0] Create Dynamic Material Instance to create Materialization Effect with changing values in the Parameters.
  (bind _returnvalue (Rendering|Material|CreateDynamicMaterialInstance (Variables|Default|GetSuspended%20Platform) 0 0 :!class /Script/Engine.PrimitiveComponent))
  (Utilities|FlowControl|Sequence
    (:then_0
      (bind (_direction _materializationz _boost _opacity) (Timeline|Materialization,%20Boost%20and%20Opacity PlayFromStart)
        (:Update
          (Rendering|Material|SetScalarParameterValue _returnvalue "Amount" _materializationz :!class /Script/Engine.MaterialInstanceDynamic)
          (Rendering|Material|SetScalarParameterValue _returnvalue "Boost" _boost :!class /Script/Engine.MaterialInstanceDynamic)
          (Rendering|Material|SetScalarParameterValue _returnvalue "Opacity" _opacity :!class /Script/Engine.MaterialInstanceDynamic))
        (:Finished
          ;;[1 1 1] Sound Effects
          (Utilities|FlowControl|Delay 2.0)
          (Components|Activation|SetActive (Variables|Default|GetS_Materialization) false false))))
    (:then_1
      (Components|Activation|SetActive (Variables|Default|GetS_Materialization) true false))))

(event EventTick
  (params (DeltaSeconds :type Float%20%28single-precision%29))
  (bind _suspended_platform (Variables|Default|GetSuspended%20Platform))
  (bind _returnvalue (Transformation|GetWorldRotation _suspended_platform))
  (bind _returnvalue_2 (Transformation|GetWorldLocation _suspended_platform))
  ;[0 1 1] Create "Sensor" that will be updated at all times. The Sensor is detecting the character "Speedster". If the Speedster is detected, the Variable will be defined according to the result.
  (bind (_outhits _returnvalue_3) (Class|KismetSystemLibrary|BoxTraceMultiforObjects _returnvalue_2 (+ _returnvalue_2 "1.000000,1.000000,1.000000") "25.000000,250.000000,450.000000" (Math|Rotator|MakeRotator (.roll _returnvalue) (- (.pitch _returnvalue) 9e+01) (.yaw _returnvalue)) (Utilities|Array|MakeArray "ObjectTypeQuery3") false 0 "None" true))
  (if _returnvalue_3
    (for _array_element _outhits
      (Utilities|Casting|CastToBP_Speedster (.HitActor (Collision|BreakHitResult _array_element))
        (:then
          (Variables|Character|SetCharacter%20Detected true))
        (:CastFailed
          (Variables|Character|SetCharacter%20Detected false))))
    (else
      ;;[1 1 1] When the Character leaves the "Sensor", the "Sphere" collision will return to normal.
      (if (Variables|Character|GetCharacter%20Detected)
        (Collision|SetCollisionResponsetoChannel (Variables|Default|GetSensor) "ECC_Pawn" (Variables|Collision|GetCollision%20Sensor))
        (Variables|Character|SetCharacter%20Detected false)
        (Utilities|FlowControl|FlipFlop
          (:B
            ;[1 0 0] After end of overlay destroy actor.
            (CallFunction|RunonServerSensor)))))))

(fn ConstructionScript)