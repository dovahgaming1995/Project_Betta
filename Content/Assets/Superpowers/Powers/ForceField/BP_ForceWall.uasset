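; Force wall actor that materializes with animated material and sound, and breaks after a set number of hits.
; Sensor overlaps route through a server RPC to a multicast that pulses the material, counts hits, then fades and destroys the wall.
; Optional server optimization skips cosmetics on the authority.
; A per-tick box trace flags BP_Speedster presence and restores the sensor's saved Pawn collision response once a detected Speedster leaves.
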(event OnComponentBeginOverlap(Sensor)
  (params (OverlappedComponent :type Primitive%20Component%20Object%20Reference) (OtherActor :type Actor%20Object%20Reference) (OtherComp :type Primitive%20Component%20Object%20Reference) (OtherBodyIndex :type Integer) (bFromSweep :type Boolean) (SweepResult :type Hit%20Result%20Structure%20%28by%20ref%29))
  ;[1 0.9952 0] When a character or any object collides with "Sensor" animate material using "Timeline" to create a weak effect in the protection generated by the wall.
  (CallFunction|RunonServerSensor))

(event Custom|Multicast_Sensor
  ;[1 0.9952 0] When a character or any object collides with "Sensor" animate material using "Timeline" to create a weak effect in the protection generated by the wall.
  ;;[1 0 0] Optimize Server? If so, "Clients" will normally follow the path. "Server" will have dematerialization and sound effects disabled.
  (if (Variables|Server|GetEnable%20Advanced%20Server%20Optimization?)
    (Networking|SwitchHasAuthority
      (:Authority
        ;[1 0 0] When the sum of collisions results in 10 the actor will be destroyed.
        (bind _output_get (Variables|Hit|SetHit (+ (Variables|Hit|GetHit) 1) :!label _label))
        (Utilities|FlowControl|Sequence
          (:then_0
            (Utilities|FlowControl|Delay 1.0)
            ;;[1 1 1] Sound Effects
            (Components|Activation|SetActive (Variables|Default|GetS_TouchingTheForce) false false))
          (:then_1
            (if (>= _output_get (Variables|Hit|GetNumber%20of%20Hits%20for%20Destroy))
              ;;[1 0 0] Optimize Server? If so, "Clients" will normally follow the path. "Server" will have dematerialization and sound effects disabled.
              (if (Variables|Server|GetEnable%20Advanced%20Server%20Optimization?)
                (Networking|SwitchHasAuthority
                  (:Authority
                    (Utilities|FlowControl|Delay 1.0)
                    (Actor|DestroyActor :!label _label_2))
                  (:Remote
                    ;;[1 1 1] Sound Effects
                    (Components|Activation|SetActive (Variables|Default|GetS_LosingForce) true false :!label _label_3)
                    (bind _losing_strength (Timeline|Losing%20Strength PlayFromStart)
                      (:Update
                        (Rendering|Material|SetScalarParameterValue (stale EventBeginPlay _returnvalue) "Opacity" _losing_strength :!class /Script/Engine.MaterialInstanceDynamic))
                      (:Finished
                        (goto _label_2)))))
                (else
                  (goto _label_3)))))))
      (:Remote
        (Utilities|FlowControl|Sequence :!label _label_4
          (:then_0
            (bind _boost (Timeline|Timeline_0 PlayFromStart)
              (:Update
                (Rendering|Material|SetScalarParameterValue (stale EventBeginPlay _returnvalue) "Boost" _boost :!class /Script/Engine.MaterialInstanceDynamic))))
          (:then_1
            ;;[1 1 1] Sound Effects
            (Components|Activation|SetActive (Variables|Default|GetS_TouchingTheForce) true false)
            (goto _label)))))
    (else
      (goto _label_4))))

(event Custom|RunOnServer_Sensor
  ;[1 0.9952 0] When a character or any object collides with "Sensor" animate material using "Timeline" to create a weak effect in the protection generated by the wall.
  (CallFunction|MulticastSensor))

(event EventBeginPlay
  ;[1 0.9765 0] Create Dynamic Material Instance to create Materialization Effect with changing values in the Parameters.
  ;;[1 1 1] Get "Sphere" collision configuration. Set Variable to save the configuration to be used in the "Sensor".
  (Variables|Vibrate|SetCollision_Sensor (Collision|GetCollisionResponsetoChannel (Variables|Default|GetSensor) "ECC_Pawn"))
  ;;[1 0 0] Optimize Server? If so, "Clients" will normally follow the path. "Server" will have materialization and sound effects disabled.
  (if (Variables|Server|GetEnable%20Advanced%20Server%20Optimization?)
    (Networking|SwitchHasAuthority
      (:Remote
        _)))
  (bind _returnvalue (Rendering|Material|CreateDynamicMaterialInstance (Variables|Default|GetForceWall) 0 "/Game/SuperPowers/Powers/ForceField/Materials/MI_Force.MI_Force" :!class /Script/Engine.PrimitiveComponent))
  (Utilities|FlowControl|Sequence
    (:then_0
      (bind (_direction _materializationz _boost _opacity) (Timeline|Materialization,%20Boost%20and%20Opacity PlayFromStart)
        (:Update
          (Rendering|Material|SetScalarParameterValue _returnvalue "Amount" _materializationz :!class /Script/Engine.MaterialInstanceDynamic)
          (Rendering|Material|SetScalarParameterValue _returnvalue "Boost" _boost :!class /Script/Engine.MaterialInstanceDynamic)
          (Rendering|Material|SetScalarParameterValue _returnvalue "Opacity" _opacity :!class /Script/Engine.MaterialInstanceDynamic))
        (:Finished
          ;;[1 1 1] Sound Effects
          (Utilities|FlowControl|Delay 2.0)
          (Components|Activation|SetActive (Variables|Default|GetS_Materialization) false false))))
    (:then_1
      (Components|Activation|SetActive (Variables|Default|GetS_Materialization) true false))))

(event EventTick
  (params (DeltaSeconds :type Float%20%28single-precision%29))
  (bind _forcewall (Variables|Default|GetForceWall))
  (bind _returnvalue (Transformation|GetWorldRotation _forcewall))
  (bind _returnvalue_2 (Transformation|GetWorldLocation _forcewall))
  ;[0 1 1] Create "Sensor" that will be updated at all times. The Sensor is detecting the character "Speedster". If the Speedster is detected, the Variable will be defined according to the result.
  (bind (_outhits _returnvalue_3) (Class|KismetSystemLibrary|BoxTraceMultiforObjects _returnvalue_2 (+ _returnvalue_2 "1.000000,1.000000,1.000000") "50.000000,650.000000,200.000000" (Math|Rotator|MakeRotator (.roll _returnvalue) (- (.pitch _returnvalue) 9e+01) (.yaw _returnvalue)) (Utilities|Array|MakeArray "ObjectTypeQuery3") false 0 "None" true))
  (if _returnvalue_3
    (for _array_element _outhits
      (Utilities|Casting|CastToBP_Speedster (.HitActor (Collision|BreakHitResult _array_element))
        (:then
          (Variables|Vibrate|SetCharacter%20Detected true))
        (:CastFailed
          (Variables|Vibrate|SetCharacter%20Detected false))))
    (else
      ;;[1 1 1] When the Character leaves the "Sensor", the "Sphere" collision will return to normal.
      (if (Variables|Vibrate|GetCharacter%20Detected)
        (Collision|SetCollisionResponsetoChannel (Variables|Default|GetSensor) "ECC_Pawn" (Variables|Vibrate|GetCollision_Sensor))
        (Variables|Vibrate|SetCharacter%20Detected false)))))

(fn ConstructionScript)