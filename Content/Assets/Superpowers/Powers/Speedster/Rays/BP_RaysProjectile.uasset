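; BP_RaysProjectile is a lightning ray projectile for the Speedster superpower that bursts on contact.
; Each Tick spawns lightning trail particles at SM_Sphere's location and yaw; with advanced server optimization, the authority skips them and deactivates the projectile sound.
; Overlaps or hits on the three spheres, or overlaps on the Sensor, route through a server event to a multicast that spawns BP_LightningBurst below the projectile and destroys it.
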(event OnComponentHit(SM_Sphere)
  (params (HitComponent :type Primitive%20Component%20Object%20Reference) (OtherActor :type Actor%20Object%20Reference) (OtherComp :type Primitive%20Component%20Object%20Reference) (NormalImpulse :type Vector :default "0, 0, 0") (Hit :type Hit%20Result%20Structure%20%28by%20ref%29))
  ;[1 0.006282 0] If something overlaps or hits "SM_Sphere, 2 and 3" or "Sensor" spawns "BP_LightningBurst" and destroys the actor.
  (CallFunction|RunonServerSensor))

(event OnComponentHit(SM_Sphere2)
  (params (HitComponent :type Primitive%20Component%20Object%20Reference) (OtherActor :type Actor%20Object%20Reference) (OtherComp :type Primitive%20Component%20Object%20Reference) (NormalImpulse :type Vector :default "0, 0, 0") (Hit :type Hit%20Result%20Structure%20%28by%20ref%29))
  ;[1 0.006282 0] If something overlaps or hits "SM_Sphere, 2 and 3" or "Sensor" spawns "BP_LightningBurst" and destroys the actor.
  (CallFunction|RunonServerSensor))

(event OnComponentBeginOverlap(SM_Sphere)
  (params (OverlappedComponent :type Primitive%20Component%20Object%20Reference) (OtherActor :type Actor%20Object%20Reference) (OtherComp :type Primitive%20Component%20Object%20Reference) (OtherBodyIndex :type Integer) (bFromSweep :type Boolean) (SweepResult :type Hit%20Result%20Structure%20%28by%20ref%29))
  ;[1 0.006282 0] If something overlaps or hits "SM_Sphere, 2 and 3" or "Sensor" spawns "BP_LightningBurst" and destroys the actor.
  (CallFunction|RunonServerSensor))

(event OnComponentBeginOverlap(SM_Sphere2)
  (params (OverlappedComponent :type Primitive%20Component%20Object%20Reference) (OtherActor :type Actor%20Object%20Reference) (OtherComp :type Primitive%20Component%20Object%20Reference) (OtherBodyIndex :type Integer) (bFromSweep :type Boolean) (SweepResult :type Hit%20Result%20Structure%20%28by%20ref%29))
  ;[1 0.006282 0] If something overlaps or hits "SM_Sphere, 2 and 3" or "Sensor" spawns "BP_LightningBurst" and destroys the actor.
  (CallFunction|RunonServerSensor))

(event OnComponentBeginOverlap(SM_Sphere3)
  (params (OverlappedComponent :type Primitive%20Component%20Object%20Reference) (OtherActor :type Actor%20Object%20Reference) (OtherComp :type Primitive%20Component%20Object%20Reference) (OtherBodyIndex :type Integer) (bFromSweep :type Boolean) (SweepResult :type Hit%20Result%20Structure%20%28by%20ref%29))
  ;[1 0.006282 0] If something overlaps or hits "SM_Sphere, 2 and 3" or "Sensor" spawns "BP_LightningBurst" and destroys the actor.
  (CallFunction|RunonServerSensor))

(event OnComponentBeginOverlap(Sensor)
  (params (OverlappedComponent :type Primitive%20Component%20Object%20Reference) (OtherActor :type Actor%20Object%20Reference) (OtherComp :type Primitive%20Component%20Object%20Reference) (OtherBodyIndex :type Integer) (bFromSweep :type Boolean) (SweepResult :type Hit%20Result%20Structure%20%28by%20ref%29))
  ;[1 0.006282 0] If something overlaps or hits "SM_Sphere, 2 and 3" or "Sensor" spawns "BP_LightningBurst" and destroys the actor.
  (CallFunction|RunonServerSensor))

(event OnComponentHit(SM_Sphere3)
  (params (HitComponent :type Primitive%20Component%20Object%20Reference) (OtherActor :type Actor%20Object%20Reference) (OtherComp :type Primitive%20Component%20Object%20Reference) (NormalImpulse :type Vector :default "0, 0, 0") (Hit :type Hit%20Result%20Structure%20%28by%20ref%29))
  ;[1 0.006282 0] If something overlaps or hits "SM_Sphere, 2 and 3" or "Sensor" spawns "BP_LightningBurst" and destroys the actor.
  (CallFunction|RunonServerSensor))

(event Custom|Multicast_Sensor
  (bind _returnvalue (Transformation|GetActorTransform))
  ;[1 0.006282 0] If something overlaps or hits "SM_Sphere, 2 and 3" or "Sensor" spawns "BP_LightningBurst" and destroys the actor.
  (Game|SpawnActorfromClass "/Game/SuperPowers/Powers/Speedster/Rays/BP_LightningBurst.BP_LightningBurst_C" (Math|Transform|MakeTransform (+ (.location _returnvalue) "0, 0,-130.000000") (.rotation _returnvalue) (.scale _returnvalue)) "Undefined" 0 0)
  (Actor|DestroyActor))

(event Custom|RunOnServer_Sensor
  ;[1 0.006282 0] If something overlaps or hits "SM_Sphere, 2 and 3" or "Sensor" spawns "BP_LightningBurst" and destroys the actor.
  (CallFunction|MulticastSensor))

(event EventTick
  (params (DeltaSeconds :type Float%20%28single-precision%29))
  (bind _sm_sphere (Variables|Default|GetSM_Sphere))
  ;[0.9595 1 0] Create Particles based on the Location and Rotation of "SM_Sphere".
  ;;[1 0 0] Optimize Server? If so, "Clients" will normally follow the path. "Server" will have particles and sound effects disabled.
  (if (Variables|Server|GetEnable%20Advanced%20Server%20Optimization?)
    (Networking|SwitchHasAuthority
      (:Authority
        ;;[1 1 1] Sound Effects
        (Components|Activation|SetActive (Variables|Default|GetS_RaysProjectile) false false))
      (:Remote
        (Effects|SpawnEmitteratLocation "/Game/SuperPowers/Powers/Speedster/Rays/Particles/P_LightningTrail.P_LightningTrail" (Transformation|GetWorldLocation _sm_sphere) (Math|Rotator|MakeRotator 0.0 0.0 (- (.yaw (Transformation|GetWorldRotation _sm_sphere)) -9e+01)) :!label _label)))
    (else
      (goto _label))))

(fn ConstructionScript)