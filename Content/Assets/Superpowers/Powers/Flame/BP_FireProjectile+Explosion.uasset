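; Fire projectile for the Flame superpower that leaves a flame trail and ends in an explosion.
; Tick spawns a fire emitter at the collision's transform, with optional server optimization skipping particles and silencing flight sound on authority.
; Collision physics starts shortly after BeginPlay.
; Low speed detonates it immediately, while projectile stop or a lifetime timeout detonates after a short delay, spawning BP_Explosion on authority and destroying the actor.
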(event OnProjectileStop(ProjectileMovement)
  (params (ImpactResult :type Hit%20Result%20Structure%20%28by%20ref%29))
  ;[1 0 0.01785] After 0.1 seconds, activate Physics Simulation and after 5 seconds or when the projectile stops, create the "BP_Explosion" and destroy the actor.
  (Variables|Projectile|SetProjectileStop true)
  (Utilities|FlowControl|Delay 0.6)
  ;;[1 1 1] Sound Effects
  (Components|Activation|SetActive (Variables|Default|GetS_FlameProjectile) false false)
  (Utilities|FlowControl|Sequence
    (:then_0
      (Networking|SwitchHasAuthority
        (:Authority
          (Game|SpawnActorfromClass "/Game/SuperPowers/Powers/Flame/BP_Explosion.BP_Explosion_C" (Transformation|GetActorTransform) "Undefined" 0 0))))
    (:then_1
      (Actor|DestroyActor))))

(event EventBeginPlay
  ;[1 0 0.01785] After 0.1 seconds, activate Physics Simulation and after 5 seconds or when the projectile stops, create the "BP_Explosion" and destroy the actor.
  (Utilities|FlowControl|Delay 0.1)
  (Physics|SetSimulatePhysics (Variables|Default|GetCollision) true)
  (Utilities|FlowControl|Delay 5.0)
  (Variables|Projectile|SetProjectileStop true)
  (Utilities|FlowControl|Delay 0.6)
  ;;[1 1 1] Sound Effects
  (Components|Activation|SetActive (Variables|Default|GetS_FlameProjectile) false false)
  (Utilities|FlowControl|Sequence
    (:then_0
      (Networking|SwitchHasAuthority
        (:Authority
          (Game|SpawnActorfromClass "/Game/SuperPowers/Powers/Flame/BP_Explosion.BP_Explosion_C" (Transformation|GetActorTransform) "Undefined" 0 0))))
    (:then_1
      (Actor|DestroyActor))))

(event EventTick
  (params (DeltaSeconds :type Float%20%28single-precision%29))
  (bind _collision (Variables|Default|GetCollision))
  (bind _returnvalue (Transformation|GetWorldRotation _collision))
  ;[0.06462 1 0] Set Location and Rotation of the Creation of Particle
  (if (not (Variables|Projectile|GetProjectileStop))
    ;;[1 0 0] Optimize Server? If so, "Clients" will normally follow the path. "Server" will have particles and sound effects disabled.
    (if (Variables|Server|GetEnable%20Advanced%20Server%20Optimization?)
      (Networking|SwitchHasAuthority
        (:Authority
          ;;[1 1 1] Sound Effects
          (Components|Activation|SetActive (Variables|Default|GetS_FlameProjectile) false false))
        (:Remote
          (Effects|SpawnEmitteratLocation "/Game/SuperPowers/Powers/Flame/Particles/P_ThrowFire.P_ThrowFire" (Transformation|GetWorldLocation _collision) (Math|Rotator|MakeRotator (.roll _returnvalue) (.pitch _returnvalue) (.yaw _returnvalue)) :!label _label)))
      (else
        (goto _label)))
    ;[0 1 0.003621] Check the projectile speed at all times. Is the speed less than or equal to 200 km / h or 124 mph? If it is less than or equal ...
    (if (<= (/ (Math|Float|Truncate (Math|Vector|VectorLength (Transformation|GetVelocity))) 28) 200)
      ;[1 0 0.01785] After 0.1 seconds, activate Physics Simulation and after 5 seconds or when the projectile stops, create the "BP_Explosion" and destroy the actor.
      ;;[1 1 1] Sound Effects
      (Components|Activation|SetActive (Variables|Default|GetS_FlameProjectile) false false)
      (Utilities|FlowControl|Sequence
        (:then_0
          (Networking|SwitchHasAuthority
            (:Authority
              (Game|SpawnActorfromClass "/Game/SuperPowers/Powers/Flame/BP_Explosion.BP_Explosion_C" (Transformation|GetActorTransform) "Undefined" 0 0))))
        (:then_1
          (Actor|DestroyActor))))))

(fn ConstructionScript)