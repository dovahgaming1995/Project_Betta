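; BP_Explosion is a short-lived explosion effect actor for the Flame superpower.
; After a brief delay on BeginPlay, a timeline grows the explosion mesh by adding its value to the current scale each update.
; When the timeline finishes, the mesh component is destroyed, and the actor follows after a further delay.
; An optional server optimization deactivates the particle and sound components where the actor has authority.
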(event EventBeginPlay
  (bind _mesh_explosion (Variables|Default|GetMesh_Explosion))
  ;[1 0 0] Optimize Server? If so, "Clients" will normally follow the path. "Server" will have particles and sound effects disabled.
  (if (Variables|Server|GetEnable%20Advanced%20Server%20Optimization?)
    (Networking|SwitchHasAuthority
      (:Authority
        (Components|Activation|SetActive (Variables|Default|GetP_Explosion) false false)
        (Components|Activation|SetActive (Variables|Default|GetS_Explosion) false false))
      (:Remote
        _)))
  (Utilities|FlowControl|Delay 0.1)
  ;[1 0.9674 0] Increase the size of the Explosion Mesh based on the values of the "Timeline" called "Scale".
  (bind _scale (Timeline|Scale PlayFromStart)
    (:Update
      (Transformation|SetWorldScale3D _mesh_explosion (+ (Transformation|GetWorldScale _mesh_explosion) _scale)))
    (:Finished
      ;[1 0 0] After the end of the "Timeline" destroy the explosion mesh. After a 2-second delay, destroy the Blueprint.
      (Components|DestroyComponent (Variables|Default|GetMesh_Explosion))
      (Utilities|FlowControl|Delay 5.0)
      (Actor|DestroyActor))))

(fn ConstructionScript)