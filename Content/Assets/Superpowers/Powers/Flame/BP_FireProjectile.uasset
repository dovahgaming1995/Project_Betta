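; BP_FireProjectile is the fire projectile of the Flame superpower, leaving a trail by spawning a throw-fire emitter at its collision every tick.
; Shortly after BeginPlay it starts blocking Pawns and simulating physics.
; On projectile stop or a timeout, the trail ends, then sound is deactivated and the actor destroyed after a brief delay.
; Optional server optimization skips particles and silences sound on the authority, leaving effects to remotes.
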(event OnProjectileStop(ProjectileMovement)
  (params (ImpactResult :type Hit%20Result%20Structure%20%28by%20ref%29))
  ;[1 0 0.01785] After 0.1s activate Simulates Physics and after 5s or when the Projectile Stops Destroy the Actor
  (Variables|Projectile|SetProjectileStop true)
  (Utilities|FlowControl|Delay 0.6)
  ;;[1 1 1] Sound Effects
  (Components|Activation|SetActive (Variables|Default|GetS_FlameProjectile) false false)
  (Actor|DestroyActor))

(event EventBeginPlay
  ;[1 0 0.01785] After 0.1s activate Simulates Physics and after 5s or when the Projectile Stops Destroy the Actor
  (Utilities|FlowControl|Delay 0.1)
  (Collision|SetCollisionResponsetoChannel (Variables|Default|GetCollision) "ECC_Pawn" "ECR_Block")
  (Physics|SetSimulatePhysics (Variables|Default|GetCollision) true)
  (Utilities|FlowControl|Delay 5.0)
  (Variables|Projectile|SetProjectileStop true)
  (Utilities|FlowControl|Delay 0.6)
  ;;[1 1 1] Sound Effects
  (Components|Activation|SetActive (Variables|Default|GetS_FlameProjectile) false false)
  (Actor|DestroyActor))

(event EventTick
  (params (DeltaSeconds :type Float%20%28single-precision%29))
  (bind _collision (Variables|Default|GetCollision))
  (bind _returnvalue (Transformation|GetWorldRotation _collision))
  ;[0.06462 1 0] Set Location and Rotation of the Creation of Particle
  (if (not (Variables|Projectile|GetProjectileStop))
    ;;[1 0 0] Optimize Server? If so, "Clients" will normally follow the path. "Server" will have particles and sound effects disabled.
    (if (Variables|Server|GetEnable%20Advanced%20Server%20Optimization?)
      (Networking|SwitchHasAuthority
        (:Authority
          ;;[1 1 1] Sound Effects
          (Utilities|FlowControl|DoOnce false
            (:Completed
              (Components|Activation|SetActive (Variables|Default|GetS_FlameProjectile) false false))))
        (:Remote
          (Effects|SpawnEmitteratLocation "/Game/SuperPowers/Powers/Flame/Particles/P_ThrowFire.P_ThrowFire" (Transformation|GetWorldLocation _collision) (Math|Rotator|MakeRotator (.roll _returnvalue) (.pitch _returnvalue) (.yaw _returnvalue)) :!label _label)))
      (else
        (goto _label)))))

(fn ConstructionScript)